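; AI controller for an enemy in the fighting game, running the BT_FightingEnemy behavior tree on possession.
; AI perception updates write a successfully sensed Player-tagged actor to the PlayerActor blackboard key and set EnemyActor with no object supplied.
; Any other perception update only prints a "Not sensed" debug message, leaving the stored target in place.
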(event OnTargetPerceptionUpdated(AIPerception)
  (params (Actor :type Actor%20Object%20Reference) (Stimulus :type AI%20Stimulus%20Structure))
  (bind _blackboard (Variables|Default|GetBlackboard))
  (if (and (Actor|ActorHasTag Actor "Player") (.bSuccessfullySensed (Utilities|Struct|BreakAIStimulus Stimulus)))
    (AI|Components|Blackboard|SetValueasObject _blackboard (Variables|Default|GetPlayerActor) Actor)
    (AI|Components|Blackboard|SetValueasObject _blackboard (Variables|Default|GetEnemyActor) 0)
    (else
      (Development|PrintString "Not sensed"))))

(event EventPossess
  (params (PossessedPawn :type Pawn%20Object%20Reference))
  (AI|RunBehaviorTree "/Game/FightingGame/AI/BT_FightingEnemy.BT_FightingEnemy"))

(fn ConstructionScript)