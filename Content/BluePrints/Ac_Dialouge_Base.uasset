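; Ac_Dialouge_Base is a base dialogue component that opens and closes a conversation UI.
; OpenConversation creates a W_DiaLouge widget with itself as owning component, adds it to the viewport and calls ProgressDialouge.
; ProgressDialouge sets the tree index to -1 and calls Dialouge, which is empty here.
; Functions for adding lines, updating the selected option, clearing or removing progress and setting the index are also empty stubs.
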(fn OpenConversation
  (bind _returnvalue (UserInterface|CreateWidget "/Game/UI/W_DiaLouge.W_DiaLouge_C" 0 self))
  (bind _output_get (Variables|Default|SetDialougeWidget _returnvalue))
  (UserInterface|Viewport|AddtoViewport _output_get 0)
  (CallFunction|ProgressDialouge))

(fn CloseConversation
  (Widget|RemovefromParent (Variables|Default|GetDialougeWidget)))

(fn ProgressDialouge
  (Variables|Default|SetDialougeTreeIndex -1)
  (CallFunction|Dialouge))

(fn Dialouge)

(fn AddDialouge
  (params (NewParam :type Text) (NewParam1 :type Text) (NewParam2 :type Text)))

(fn UpdataSelectedOption)

(fn ClearDialougeProgress)

(fn RemoveDialogueProgress)

(fn SetDialogTreeindex)