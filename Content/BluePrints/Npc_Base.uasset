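; Base Blueprint for NPCs, providing a name label that signals when the character can be interacted with.
; The construction script writes the Name variable into a TextRender component, and the Showinteractable event toggles that text's visibility from a boolean.
; When a conversation closes, the Converdationclosed event notifies the stored InteractInstigator.
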(event EventShowinteractable
  (params (CanSHowInteract :type Boolean))
  (if CanSHowInteract
    (Rendering|SetVisibility (Variables|Default|GetTextRender) true false)
    (else
      (Rendering|SetVisibility (Variables|Default|GetTextRender) false false))))

(event EventConverdationclosed
  (Class|BPIINteractable|Converdationclosed(Message) (Variables|Default|GetInteractInstigator)))

(fn ConstructionScript
  (Rendering|Components|TextRender|SetText (Variables|Default|GetTextRender) (Variables|Default|GetName)))