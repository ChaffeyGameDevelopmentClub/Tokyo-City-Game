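; Test NPC Blueprint that reacts to being hit and starts a dialogue when interacted with.
; On the first hit only, gated by a HitAlready flag, it sends InteractMessage and SetControlsMessage(false) to the other actor and prints a debug greeting.
; The Interact event opens a conversation through its TextDialouge reference.
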(event EventInteract
  (params (instigator :type Actor%20Object%20Reference))
  (Default|OpenConversation (Variables|Default|GettextDialouge)))

(event Collision|EventHit
  (params (MyComp :type Primitive%20Component%20Object%20Reference) (Other :type Actor%20Object%20Reference) (OtherComp :type Primitive%20Component%20Object%20Reference) (bSelfMoved :type Boolean) (HitLocation :type Vector :default "0, 0, 0") (HitNormal :type Vector :default "0, 0, 0") (NormalImpulse :type Vector :default "0, 0, 0") (Hit :type Hit%20Result%20Structure%20%28by%20ref%29))
  (if (not (Variables|Default|GetHitAlready))
    (Class|BPIINteractable|Interact(Message) self Other)
    (Class|BPIINteractable|SetControls(Message) Other false)
    (Variables|Default|SetHitAlready true)
    (Development|PrintString "Hello")))

(fn ConstructionScript)