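; Dialogue component base that opens a dialogue widget and notifies its owner when the conversation closes.
; DiaLogue is an empty hook, presumably overridden to script conversations through AddDialogue calls.
; Each choice is stored by step index, then DiaLogue replays from the start: AddDialogue returns saved choices and displays unanswered steps.
; Progress can be rolled back, or cleared when the dialogue tree index changes.
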(fn OpenConversation
  (bind _returnvalue (UserInterface|CreateWidget "/Game/UI/W_DiaLouge.W_Dialouge_C" 0 self))
  (bind _output_get (Variables|Default|SetDialogueWidget _returnvalue))
  (UserInterface|Viewport|AddtoViewport _output_get 0)
  (CallFunction|ProgressDialogue))

(fn CloseConversation
  (Widget|RemovefromParent (Variables|Default|GetDialogueWidget))
  (Class|BPIINteractable|Converdationclosed(Message) (Components|GetOwner)))

(fn ProgressDialogue
  (Variables|Default|SetDialougeindex -1)
  (CallFunction|DiaLogue))

(fn DiaLogue)

(fn AddDialogue
  (params (Speaker :type Text) (Dialouge :type Text) (OPtionsText :type Array%20of%20Texts))
  (bind _dialogueprogess (Variables|Default|GetDialogueProgess))
  (bind _dialougeindex (Variables|Default|GetDialougeindex))
  (bind (_value _returnvalue) (Utilities|Map|Find _dialogueprogess _dialougeindex))
  (Math|Integer|IncrementInt (Variables|Default|GetDialougeindex)
    (:%20%20
      (if _returnvalue
        (return "NewEnumerator0" _value)
        (else
          (Default|UpdateDiaLogueText (Variables|Default|GetDialogueWidget) (Variables|Default|GetDialougeindex) Speaker Dialouge OPtionsText)
          (return "NewEnumerator1" 0))))))

(fn UpdateSelectedOption
  (params (ProgressIndex :type Integer%20%28by%20ref%29) (OptionIndex :type Integer%20%28by%20ref%29))
  (Utilities|Map|Add (Variables|Default|GetDialogueProgess) ProgressIndex OptionIndex)
  (CallFunction|ProgressDialogue))

(fn ClearDialogueProgress
  (Utilities|Map|Clear (Variables|Default|GetDialogueProgess)))

(fn RemoveDialogueProgess
  (params (ProgessStep :type Integer))
  (for _index (range 0 ProgessStep)
    (Utilities|Map|Remove (Variables|Default|GetDialogueProgess) (- (Variables|Default|GetDialougeindex) _index))))

(fn SetDialogTreeindex
  (params (DialogueTreeIndex :type Integer))
  (Variables|Default|SetDialougeTreeindex DialogueTreeIndex)
  (CallFunction|ClearDialogueProgress))