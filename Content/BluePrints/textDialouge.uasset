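; A dialogue Blueprint that overrides a parent dialogue system to play a short scolding line from "God".
; DiaLogue branches on the dialogue tree index and chains AddDialogue nodes; after the reply it trims progress, closes the conversation and calls Open Level with no level name set.
; An unconnected branching "Bob" conversation, which can advance the tree index, never runs.
; CloseConversation only calls its parent, and NewFunction is empty.
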(fn DiaLogue
  (|CallParentFunction)
  (switch int (Variables|Default|GetDialougeTreeindex)
    (:0
      (bind _state (CallFunction|AddDialogue "God" "What the hell you think your doing steping on mt house like that?!" (Utilities|Array|MakeArray "sorry")))
      (switch Utilities|FlowControl|Switch|SwitchonEnum_State _state
        (:NewEnumerator0
          (CallFunction|RemoveDialogueProgess 2)
          (CallFunction|CloseConversation)
          (Game|OpenLevel(byName) "None"))))))

(fn NewFunction)

(fn CloseConversation
  (|CallParentFunction))